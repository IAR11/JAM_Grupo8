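; BoxFallen_BP is a trigger volume that kills the DeafCharacterBP on overlap, likely marking a fall hazard.
; Overlap plays a 2D death sound and shows a FadeToBlack widget, then after a short delay destroys the character and removes all widgets.
; The construction script sizes the box from the BoxExtent variable.
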(event `self.Box.OnComponentBeginOverlap`
  (params (OverlappedComponent :type "PrimitiveComponent Object Reference") (OtherActor :type "Actor Object Reference") (OtherComp :type "PrimitiveComponent Object Reference") (OtherBodyIndex :type Integer) (bFromSweep :type Boolean) (SweepResult :type "HitResult Structure (by ref)"))
  (bind _asdeaf_character_bp (cast `/Game/DeafPersonBP/DeafCharacterBP` OtherActor))
  (`GameplayStatics.PlaySound2D` "/Game/Audios/Death.Death" 1.0 1.0 0.0 null null)
  (bind _returnvalue (`|CreateWidget` "/Game/Blueprints/FadeToBlack.FadeToBlack_C"))
  (`/Game/Blueprints/FadeToBlack.FadeToBlack` _returnvalue)
  (`UserWidget.AddToViewport` _returnvalue 0)
  (`KismetSystemLibrary.Delay` 1.5)
  (`self.K2_DestroyActor` _asdeaf_character_bp)
  (`WidgetLayoutLibrary.RemoveAllWidgets`))

(fn `UserConstructionScript`
  (`BoxComponent.SetBoxExtent` (`self.Box`) (`self.BoxExtent`) true))