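; Platform actor that moves its Platform component between two marker components in the level.
; On BeginPlay, it sets the PlatformMovement timeline's play rate from MoveRate and plays it from the start.
; Each timeline update uses the Alpha track to lerp the world location from StartMovement to EndMovement1, without sweep.
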(event `self.ReceiveBeginPlay`
  ;[1 1 1] Movimiento Plataforma
  ;;[1 1 1] Velocidad Plataforma
  (`TimelineComponent.SetPlayRate` (`self.PlatformMovement`) (`self.MoveRate`))
  (bind (_direction _alpha) (`Timeline|PlatformMovement` :!via `PlayFromStart`)
    (:`Update`
      (`SceneComponent.K2_SetWorldLocation` (`self.Platform `) (`KismetMathLibrary.VLerp` (`SceneComponent.K2_GetComponentLocation` (`self.StartMovement`)) (`SceneComponent.K2_GetComponentLocation` (`self.EndMovement1`)) _alpha) false false))))

(fn `UserConstructionScript`)