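; Moving platform actor that travels to an end point while a Deaf_Character is inside its trigger box and travels back when that character leaves.
; Overlap events play or reverse a timeline at a rate set by Duration, lerping the platform's relative location from its BeginPlay start to EndLocation.
; The construction script applies mesh, scale and rotation to both the platform and an end reference mesh placed at EndLocation, previewing the destination.
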(event `self.ReceiveBeginPlay`
  (set `self.StartLocation` (`SceneComponent.RelativeLocation` (`self.Platform`))))

(event `self.Box.OnComponentBeginOverlap`
  (params (OverlappedComponent :type "PrimitiveComponent Object Reference") (OtherActor :type "Actor Object Reference") (OtherComp :type "PrimitiveComponent Object Reference") (OtherBodyIndex :type Integer) (bFromSweep :type Boolean) (SweepResult :type "HitResult Structure (by ref)"))
  (cast `/Game/NoTocar/Deaf_Character` OtherActor)
  (`TimelineComponent.SetPlayRate` (`self.MovePlatform`) (/ 1.0 (`self.Duration`)))
  (bind (_direction _movetrack) (`Timeline|MovePlatform` :!label _label)
    (:`Update`
      (`SceneComponent.K2_SetRelativeLocation` (`self.Platform`) (`KismetMathLibrary.VLerp` (`self.StartLocation`) (`self.End Location`) _movetrack) false false))))

(event `self.Box.OnComponentEndOverlap`
  (params (OverlappedComponent :type "PrimitiveComponent Object Reference") (OtherActor :type "Actor Object Reference") (OtherComp :type "PrimitiveComponent Object Reference") (OtherBodyIndex :type Integer))
  (cast `/Game/NoTocar/Deaf_Character` OtherActor)
  (`TimelineComponent.SetPlayRate` (`self.MovePlatform`) (/ 1.0 (`self.Duration`)))
  (goto _label :!via `Reverse`))

(fn `UserConstructionScript`
  (bind _endreference (`self.EndReference`))
  (bind _platformmesh (`self.PlatformMesh`))
  (bind _platform (`self.Platform`))
  (`StaticMeshComponent.SetStaticMesh` _platform _platformmesh)
  (`StaticMeshComponent.SetStaticMesh` _endreference _platformmesh)
  (`SceneComponent.SetRelativeScale3D` _platform (`self.Scale`))
  (`SceneComponent.SetRelativeScale3D` _endreference (`self.Scale`))
  (`SceneComponent.K2_SetRelativeRotation` _endreference (`self.Rotation`) false false)
  (`SceneComponent.K2_SetRelativeRotation` _platform (`self.Rotation`) false false)
  (`SceneComponent.K2_SetRelativeLocation` _endreference (`self.End Location`) false false))