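; HeatingPlatform_BP is a platform that heats up when the player touches it, then temporarily disappears.
; Player overlap on Cube_Trigger starts a timeline, paced by SpeedRate, that lerps the Color of a dynamic material from InicialColor to EndColor.
; When it finishes, the cube loses collision and visibility for a fixed delay, then restores both and the initial color.
; A DoOnce blocks retriggering until that reset.
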(event `self.ReceiveBeginPlay`
  (bind _returnvalue (`KismetMaterialLibrary.CreateDynamicMaterialInstance` "/Game/Assets/Materials/Heating_M.Heating_M"))
  (bind _output_get (set `self.Heating_M` _returnvalue))
  (`PrimitiveComponent.SetMaterial` (`self.Cube`) 0 _output_get)
  (`TimelineComponent.SetPlayRate` (`self.Heating_Timeline`) (`self.Speed_Rate`))
  (`MaterialInstanceDynamic.SetVectorParameterValue` (`self.Heating_M`) "Color" (`self.Inicial_Color`)))

(event `self.Cube_Trigger.OnComponentBeginOverlap`
  (params (OverlappedComponent :type "PrimitiveComponent Object Reference") (OtherActor :type "Actor Object Reference") (OtherComp :type "PrimitiveComponent Object Reference") (OtherBodyIndex :type Integer) (bFromSweep :type Boolean) (SweepResult :type "HitResult Structure (by ref)"))
  (if (== OtherActor (`GameplayStatics.GetPlayerCharacter` 0))
    (`/Engine/EditorBlueprintResources/StandardMacros.DoOnce` false :!label _label
      (:`Completed`
        (bind (_direction _alpha) (`Timeline|Heating_Timeline` :!via `PlayFromStart`)
          (:`Update`
            (`MaterialInstanceDynamic.SetVectorParameterValue` (`self.Heating_M`) "Color" (`KismetMathLibrary.LinearColorLerp` (`self.Inicial_Color`) (`self.End_Color`) _alpha)))
          (:`Finished`
            (`PrimitiveComponent.SetCollisionEnabled` (`self.Cube`) "NoCollision")
            (`SceneComponent.SetVisibility` (`self.Cube`) false false)
            (`KismetSystemLibrary.Delay` 3.0)
            (`PrimitiveComponent.SetCollisionEnabled` (`self.Cube`) "QueryAndPhysics")
            (`SceneComponent.SetVisibility` (`self.Cube`) true false)
            (`MaterialInstanceDynamic.SetVectorParameterValue` (`self.Heating_M`) "Color" (`self.Inicial_Color`))
            (goto _label :!via `Reset`)))))))

(fn `UserConstructionScript`)