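; FlipFlop_BP is a platform that toggles between solid and non-solid each time its CharacterJump event fires.
; The event inverts the Visible flag and calls SetVisibility, which switches the Platform between visible and invisible materials and enables or disables its collision.
; The construction script calls the same function, so the initial state follows the Visible value.
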(event `/Game/Blueprints_Platform/CharacterInterface_BP.Character_Jump`
  (set `self.Visible` (not (`self.Visible`)))
  (`self.Set_Visibility`))

(fn `Set_Visibility`
  (bind _platform (`self.Platform`))
  (bind _platform_2 (`self.Platform`))
  (if (`self.Visible`)
    (`PrimitiveComponent.SetMaterial` _platform 0 (`self.VisibleMat`))
    (`PrimitiveComponent.SetCollisionEnabled` _platform "QueryAndPhysics")
    (else
      (`PrimitiveComponent.SetMaterial` _platform_2 0 (`self.InvisibleMat`))
      (`PrimitiveComponent.SetCollisionEnabled` _platform_2 "NoCollision"))))

(fn `UserConstructionScript`
  (`self.Set_Visibility`))